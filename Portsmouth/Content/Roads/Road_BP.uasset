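; Spline-driven road actor that builds a two-lane pavement with two sidewalk meshes along RoadSpline.
; The Construction Script divides the spline length by MeshLength and adds three collidable spline mesh components per segment.
; Each takes world-space start and end points from distances along the spline, with tangents from spline direction times TangentScale.
; The event graph holds no active logic.
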(fn `UserConstructionScript`
  (bind _roadspline (`self.RoadSpline`))
  (bind _tangentscale (`self.TangentScale`))
  (bind _meshlength (`self.MeshLength`))
  (for _index (range (+ (`.ReturnValue` (`KismetMathLibrary.FMod` (`SplineComponent.GetSplineLength` _roadspline) _meshlength)) 1))
    (bind _returnvalue (`AddComponent|Spline Mesh Component_1` :`bManualAttachment` true))
    (`PrimitiveComponent.SetCollisionEnabled` _returnvalue "QueryAndPhysics")
    (`StaticMeshComponent.SetStaticMesh` _returnvalue "/Game/Roads/Meshes/sm_road.sm_road_pavement_two_lane_v1")
    (bind _returnvalue_2 (* _index _meshlength))
    (bind _returnvalue_3 (`SplineComponent.GetLocationAtDistanceAlongSpline` _roadspline _returnvalue_2 "World"))
    (bind _returnvalue_4 (* (`SplineComponent.GetDirectionAtDistanceAlongSpline` _roadspline _returnvalue_2 "World") _tangentscale))
    (bind _returnvalue_5 (+ _returnvalue_2 _meshlength))
    (bind _returnvalue_6 (`SplineComponent.GetLocationAtDistanceAlongSpline` _roadspline _returnvalue_5 "World"))
    (bind _returnvalue_7 (* (`SplineComponent.GetDirectionAtDistanceAlongSpline` _roadspline _returnvalue_5 "World") _tangentscale))
    (`SplineMeshComponent.SetStartAndEnd` _returnvalue _returnvalue_3 _returnvalue_4 _returnvalue_6 _returnvalue_7 true)
    (bind _returnvalue_8 (`AddComponent|SplineMeshComponent_15400` :`bManualAttachment` true))
    (`PrimitiveComponent.SetCollisionEnabled` _returnvalue_8 "QueryAndPhysics")
    (`StaticMeshComponent.SetStaticMesh` _returnvalue_8 "/Game/Roads/Meshes/sm_road.sm_road_sidewalk_v1")
    (`SplineMeshComponent.SetStartAndEnd` _returnvalue_8 _returnvalue_3 _returnvalue_4 _returnvalue_6 _returnvalue_7 true)
    (bind _returnvalue_9 (`AddComponent|SplineMeshComponent_15409` :`bManualAttachment` true))
    (`PrimitiveComponent.SetCollisionEnabled` _returnvalue_9 "QueryAndPhysics")
    (`StaticMeshComponent.SetStaticMesh` _returnvalue_9 "/Game/Roads/Meshes/sm_road_sidewalk_left.sm_road_sidewalk_left")
    (`SplineMeshComponent.SetStartAndEnd` _returnvalue_9 _returnvalue_3 _returnvalue_4 _returnvalue_6 _returnvalue_7 true)))